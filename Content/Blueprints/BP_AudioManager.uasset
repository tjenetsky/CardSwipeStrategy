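; BP_AudioManager controls category volumes for Music, SFX and VoiceOver and plays background music.
; BeginPlay sets the base sound mix and applies each saved volume variable as a class override.
; ChangeVolumeLevel stores the new level for the chosen category and reapplies its override immediately.
; PlayBackgroundMusic looks up the requested track in a map, fading out any playing music before fading the new one in.
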(event Custom|ChangeVolumeLevel
  (params (VolumeLevel :type Float%20%28double-precision%29) (AudioSetting :type E_AudioSettings%20Enum :default "NewEnumerator0"))
  (Variables|Volume|SetVolumeLevel VolumeLevel)
  (switch Utilities|FlowControl|Switch|SwitchonE_AudioSettings AudioSetting
    (:NewEnumerator2
      (Variables|SoundClasses|SetAffectedSoundClass "/Game/Audio/SoundClasses/Music.Music")
      (Variables|Volume|SetMusicVolume (Variables|Volume|GetVolumeLevel)))
    (:NewEnumerator1
      (Variables|SoundClasses|SetAffectedSoundClass "/Game/Audio/SoundClasses/SFX.SFX")
      (Variables|Volume|SetSFXVolume (Variables|Volume|GetVolumeLevel)))
    (:NewEnumerator3
      (Variables|SoundClasses|SetAffectedSoundClass "/Game/Audio/SoundClasses/VoiceOver.VoiceOver")
      (Variables|Volume|SetVoiceOverVolume (Variables|Volume|GetVolumeLevel))))
  (Audio|SetSoundMixClassOverride (Variables|SoundClasses|GetBaseSoundMix) (Variables|SoundClasses|GetAffectedSoundClass) (Variables|Volume|GetVolumeLevel) 1.0 0.0 true))

(event Custom|Play%20Background%20Music
  (params (MusicTrack :type E_MusicTracks%20Enum :default "NewEnumerator0"))
  (Variables|Default|SetCurrentMusicTrack MusicTrack)
  (if (Audio|Components|Audio|IsPlaying (Variables|Default|GetBackgroundMusic))
    (Audio|Components|Audio|FadeOut (Variables|Default|GetBackgroundMusic) 2.0 0.0 "Linear" :!class /Script/Engine.AudioComponent)
    (Utilities|FlowControl|Delay 2.0))
  (Audio|Components|Audio|SetSound (Variables|Default|GetBackgroundMusic) (.Value (Utilities|Map|Find (Variables|Default|GetBackgroundMusicTracks) (Variables|Default|GetCurrentMusicTrack))))
  (Audio|Components|Audio|FadeIn (Variables|Default|GetBackgroundMusic) 2.0 1.0 0.0 "Linear" :!class /Script/Engine.AudioComponent))

(event EventBeginPlay
  (Class|GameplayStatics|SetBaseSoundMix (Variables|SoundClasses|GetBaseSoundMix))
  (bind _output_get (Variables|SoundClasses|SetAffectedSoundClass "/Game/Audio/SoundClasses/Music.Music"))
  (Audio|SetSoundMixClassOverride (Variables|SoundClasses|GetBaseSoundMix) _output_get (Variables|Volume|GetMusicVolume) 1.0 0.0 true)
  (bind _output_get_2 (Variables|SoundClasses|SetAffectedSoundClass "/Game/Audio/SoundClasses/SFX.SFX"))
  (Audio|SetSoundMixClassOverride (Variables|SoundClasses|GetBaseSoundMix) _output_get_2 (Variables|Volume|GetSFXVolume) 1.0 0.0 true)
  (bind _output_get_3 (Variables|SoundClasses|SetAffectedSoundClass "/Game/Audio/SoundClasses/VoiceOver.VoiceOver"))
  (Audio|SetSoundMixClassOverride (Variables|SoundClasses|GetBaseSoundMix) _output_get_3 (Variables|Volume|GetVoiceOverVolume) 1.0 0.0 true))

(fn ConstructionScript)