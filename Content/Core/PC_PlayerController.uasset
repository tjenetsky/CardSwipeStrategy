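; Player controller that owns the game's UI, creating the Main, Transition, Menu and Fade widgets and showing the mouse cursor.
; ToggleMenu swaps visibility between screens and tracks the current and exiting menu, which Escape uses to open or back out of the menu.
; Development builds also cache the game mode and mute audio.
; Debug keys print or alter game mode state such as conditions, metrics and years in power, and refresh UI.
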(event EventBeginPlay
  (if (Utilities|Enum|Equal(Enum) (Class|KismetSystemLibrary|GetBuildConfiguration) "Development")
    (CallFunction|SetupDebuggingLogic)
    (CallFunction|CreateWidgets)
    (Variables|Default|SetbShowMouseCursor true)
    (Development|PrintString "We are in development mode!" true true "(R=1.000000,G=0.710700,B=0.151169,A=1.000000)")
    (else
      (CallFunction|CreateWidgets)
      (Variables|Default|SetbShowMouseCursor true)
      (Development|PrintString "We are in shipping mode!" true true "(R=0.155584,G=1.000000,B=0.160878,A=1.000000)"))))

(event Custom|Setup%20Debugging%20Logic
  (bind _asgm_game_mode (Utilities|Casting|CastToGM_GameMode (Game|GetGameMode)))
  (Variables|References|SetGameMode _asgm_game_mode)
  (Utilities|FlowControl|DelayUntilNextTick)
  (CallFunction|DEBUGMuteAudio))

(event Input|KeyboardEvents|DebugKeyD
  (params (Key :type Key%20Structure :default "None") (ActionValue :type Input%20Action%20Value%20Structure))
  (:Pressed
    (Default|DEBUGModifyMetricValues (Variables|References|GetGameMode) "NewEnumerator0")))

(event Input|KeyboardEvents|DebugKeyO
  (params (Key :type Key%20Structure :default "None") (ActionValue :type Input%20Action%20Value%20Structure))
  (:Pressed
    (for _array_element (Variables|/Game/UI/WBP_Main.WBP_Main_C|GetMetricWidgets (Variables|References|GetWBP_Main))
      (Widget|SetVisibility (Variables|/Game/UI/WBP_Metric.WBP_Metric_C|GetTXT_Value _array_element) "SelfHitTestInvisible"))))

(event Input|KeyboardEvents|DebugKeyH
  (params (Key :type Key%20Structure :default "None") (ActionValue :type Input%20Action%20Value%20Structure))
  (:Pressed
    (Default|UpdateHighScores (Variables|References|GetWBP_Menu))))

(event Input|KeyboardEvents|DebugKeyN
  (params (Key :type Key%20Structure :default "None") (ActionValue :type Input%20Action%20Value%20Structure))
  (:Pressed
    (Default|DEBUGCheckCharacterNames (Variables|References|GetGameMode))))

(event Input|KeyboardEvents|DebugKeyQ
  (params (Key :type Key%20Structure :default "None") (ActionValue :type Input%20Action%20Value%20Structure))
  (:Pressed
    (CallFunction|DEBUGMuteAudio)))

(event Input|KeyboardEvents|DebugKeyP
  (params (Key :type Key%20Structure :default "None") (ActionValue :type Input%20Action%20Value%20Structure))
  (:Pressed
    (Default|DEBUGCheckCardProbability (Variables|References|GetGameMode) "daily_games_attend")))

(event Input|KeyboardEvents|DebugKeyC
  (params (Key :type Key%20Structure :default "None") (ActionValue :type Input%20Action%20Value%20Structure))
  (:Pressed
    (for _array_element (Variables|/Game/Core/GM_GameMode.GM_GameMode_C|GetActiveConditions (Variables|References|GetGameMode))
      (Development|PrintString (Utilities|String|ToString(Name) _array_element) true true "(R=0.631481,G=0.179846,B=1.000000,A=1.000000)" 2e+01))))

(event Input|KeyboardEvents|DebugKeyA
  (params (Key :type Key%20Structure :default "None") (ActionValue :type Input%20Action%20Value%20Structure))
  (:Pressed
    (for _array_element (Variables|/Game/Core/GM_GameMode.GM_GameMode_C|GetAllConditions (Variables|References|GetGameMode))
      (Development|PrintString (Utilities|String|ToString(Name) _array_element) true true "(R=0.631481,G=0.179846,B=1.000000,A=1.000000)" 2e+01))))

(event Input|KeyboardEvents|DebugKeyM
  (params (Key :type Key%20Structure :default "None") (ActionValue :type Input%20Action%20Value%20Structure))
  (:Pressed
    (bind (_senatepoints _peoplepoints _armypoints _wealthpoints) (Class|BPIGameMode|GetCurrentMetricValues(Message) (Game|GetGameMode)))
    (for _array_element (Utilities|Array|MakeArray _senatepoints _peoplepoints _armypoints _wealthpoints)
      (Development|PrintString (Utilities|String|ToString(Integer) _array_element) true true "(R=0.459297,G=0.351329,B=1.000000,A=1.000000)"))))

(event Input|KeyboardEvents|DebugKeyY
  (params (Key :type Key%20Structure :default "None") (ActionValue :type Input%20Action%20Value%20Structure))
  (bind _gamemode (Variables|References|GetGameMode))
  (:Pressed
    (bind _output_get (Variables|/Game/Core/GM_GameMode.GM_GameMode_C|SetYearsInPower _gamemode (+ (Variables|/Game/Core/GM_GameMode.GM_GameMode_C|GetYearsInPower _gamemode) 5)))
    (Default|UpdateYearLength (Variables|/Game/Core/GM_GameMode.GM_GameMode_C|GetWBP_Main (Variables|References|GetGameMode)) _output_get)))

(event Input|KeyboardEvents|DebugKeyB
  (params (Key :type Key%20Structure :default "None") (ActionValue :type Input%20Action%20Value%20Structure))
  (:Pressed
    (Default|UpdateActiveBoonsList (Variables|References|GetWBP_Menu))))

(event EventPlayScreenFade
  (params (FadeToBlack :type Boolean))
  (if FadeToBlack
    (Default|FadetoBlack (Variables|References|GetWBP_Fade) 1.0)
    (else
      (Default|FadefromBlack (Variables|References|GetWBP_Fade) 1.0))))

(event EventToggleMenu
  (params (MenuExiting :type E_UIMenus%20Enum :default "NewEnumerator0") (MenuEntering :type E_UIMenus%20Enum :default "NewEnumerator0"))
  (Variables|Default|SetMenuExiting MenuExiting)
  (Variables|Default|SetMenuEntering MenuEntering)
  (switch Utilities|FlowControl|Switch|SwitchonE_UIMenus (Variables|Default|GetMenuExiting)
    (:NewEnumerator0
      (Widget|SetVisibility (Variables|References|GetWBP_Main) "Hidden")
      (switch Utilities|FlowControl|Switch|SwitchonE_UIMenus (Variables|Default|GetMenuEntering)
        (:NewEnumerator1
          (Widget|SetVisibility (Variables|References|GetWBP_Transition) "SelfHitTestInvisible")
          (Default|TransitionScreenEntered (Variables|References|GetWBP_Transition))
          (Variables|Default|SetCurrentMenu "NewEnumerator1"))
        (:NewEnumerator2
          (Widget|SetVisibility (Variables|References|GetWBP_Menu) "SelfHitTestInvisible")
          (Default|MenuEntered (Variables|References|GetWBP_Menu))
          (Variables|Default|SetCurrentMenu "NewEnumerator2"))))
    (:NewEnumerator1
      (Widget|SetVisibility (Variables|References|GetWBP_Transition) "Hidden")
      (switch Utilities|FlowControl|Switch|SwitchonE_UIMenus (Variables|Default|GetMenuEntering)
        (:NewEnumerator0
          (Widget|SetVisibility (Variables|References|GetWBP_Main) "Visible")
          (Variables|Default|SetCurrentMenu "NewEnumerator0"))
        (:NewEnumerator2
          (Widget|SetVisibility (Variables|References|GetWBP_Menu) "Visible")
          (Default|MenuEntered (Variables|References|GetWBP_Menu))
          (Variables|Default|SetCurrentMenu "NewEnumerator2"))))
    (:NewEnumerator2
      (Widget|SetVisibility (Variables|References|GetWBP_Menu) "Hidden")
      (switch Utilities|FlowControl|Switch|SwitchonE_UIMenus (Variables|Default|GetMenuEntering)
        (:NewEnumerator0
          (Widget|SetVisibility (Variables|References|GetWBP_Main) "Visible")
          (Variables|Default|SetCurrentMenu "NewEnumerator0"))
        (:NewEnumerator1
          (Widget|SetVisibility (Variables|References|GetWBP_Transition) "SelfHitTestInvisible")
          (Variables|Default|SetCurrentMenu "NewEnumerator1"))))))

(event Input|KeyboardEvents|Escape
  (params (Key :type Key%20Structure :default "None"))
  (bind _wbp_menu (Variables|References|GetWBP_Menu))
  (bind _menubuttons (Variables|/Game/UI/WBP_Menu.WBP_Menu_C|GetMenuButtons _wbp_menu))
  (bind _output (Utilities|Array|Get(acopy) _menubuttons))
  (:Pressed
    (switch Utilities|FlowControl|Switch|SwitchonE_UIMenus (Variables|Default|GetCurrentMenu)
      (:NewEnumerator0
        (CallFunction|ToggleMenu "NewEnumerator0" "NewEnumerator2"))
      (:NewEnumerator2
        (switch Utilities|FlowControl|Switch|SwitchonE_UIMenus (Variables|Default|GetMenuExiting)
          (:NewEnumerator0
            (Default|ButtonHovered _output)
            (Default|ButtonClicked _output)
            (CallFunction|ToggleMenu "NewEnumerator2" "NewEnumerator0"))
          (:NewEnumerator1
            (CallFunction|ToggleMenu "NewEnumerator2" "NewEnumerator1")
            (Default|UnselectMenuButtons (Variables|References|GetWBP_Transition))))))))

(fn ConstructionScript)

(fn CreateWidgets
  (bind _returnvalue (UserInterface|CreateWidget "/Game/UI/WBP_Main.WBP_Main_C" self))
  (bind _output_get (Variables|References|SetWBP_Main _returnvalue))
  (UserInterface|Viewport|AddtoViewport _output_get 0)
  (bind _returnvalue_2 (UserInterface|CreateWidget "/Game/UI/WBP_Transition.WBP_Transition_C" self))
  (bind _output_get_2 (Variables|References|SetWBP_Transition _returnvalue_2))
  (UserInterface|Viewport|AddtoViewport _output_get_2 1)
  (Widget|SetVisibility (Variables|References|GetWBP_Transition) "Hidden")
  (bind _returnvalue_3 (UserInterface|CreateWidget "/Game/UI/WBP_Menu.WBP_Menu_C" self))
  (bind _output_get_3 (Variables|References|SetWBP_Menu _returnvalue_3))
  (UserInterface|Viewport|AddtoViewport _output_get_3 2)
  (Widget|SetVisibility (Variables|References|GetWBP_Menu) "Hidden")
  (bind _returnvalue_4 (UserInterface|CreateWidget "/Game/UI/WBP_Fade.WBP_Fade_C" self))
  (bind _output_get_4 (Variables|References|SetWBP_Fade _returnvalue_4))
  (UserInterface|Viewport|AddtoViewport _output_get_4 3)
  (Variables|Default|SetMenuExiting "NewEnumerator0"))

(fn DEBUGMuteAudio
  (bind _returnvalue (Actor|GetActorOfClass "/Game/Blueprints/BP_AudioManager.BP_AudioManager_C"))
  (bind _output_get (Variables|References|SetBP_AudioManager _returnvalue))
  (Default|ChangeVolumeLevel _output_get 0.0 "NewEnumerator2")
  (Default|ChangeVolumeLevel (Variables|References|GetBP_AudioManager) 0.0 "NewEnumerator1")
  (Default|ChangeVolumeLevel (Variables|References|GetBP_AudioManager) 0.0 "NewEnumerator3"))

(fn SwitchMenus
  (params (MenuExiting :type E_UIMenus%20Enum :default "NewEnumerator0") (NewMenu :type E_UIMenus%20Enum :default "NewEnumerator0")))

(fn GetCurrentMenu
  (return (Variables|Default|GetCurrentMenu)))

(fn GetMenuReferences
  (return (Variables|References|GetWBP_Main) (Variables|References|GetWBP_Transition) (Variables|References|GetWBP_Menu)))